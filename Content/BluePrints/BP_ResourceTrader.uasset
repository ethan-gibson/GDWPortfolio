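; BP_ResourceTrader is an AI-moved pawn that makes one round trip between an origin town and a destination town to trade resources.
; Its Move event chains two AIMoveTo calls, calling TransferResources on each successful arrival and setting IsReturning to mark the leg.
; After the return transfer it notifies the origin town through HandleTraderDestroyed and destroys itself.
; Failed moves have no handling.
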(event EventMove
  (bind _origintown (Variables|Default|GetOriginTown))
  (Variables|Default|SetisReturning false)
  (AI|AIMoveTo self (Transformation|GetActorLocation (Variables|Default|GetDestinationTown)) 0 5.0 false
    (:OnSuccess
      (Class|ResourceTrader|TransferResources)
      (Variables|Default|SetisReturning true)
      (AI|AIMoveTo self (Transformation|GetActorLocation _origintown) 0 5.0 false
        (:OnSuccess
          (Class|ResourceTrader|TransferResources)
          (Class|Town|HandleTraderDestroyed _origintown self)
          (Actor|DestroyActor))))))

(fn ConstructionScript)